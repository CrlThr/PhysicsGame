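; Chest target for arrow shooting that opens its lid and raises a target when StartSequence is called.
; Delayed, chained timelines rotate the lid, then lift the target; TargetSpawn finishing asks BP_ChestTargetManager for a random chest target.
; An overlapping BP_Arrow destroys the target and reverses TargetSpawn, whose Finished output calls the manager again.
; The lid has no closing logic, and other overlaps only print a debug string.
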(event OnComponentBeginOverlap(Collision)
  (params (OverlappedComponent :type Primitive%20Component%20Object%20Reference) (OtherActor :type Actor%20Object%20Reference) (OtherComp :type Primitive%20Component%20Object%20Reference) (OtherBodyIndex :type Integer) (bFromSweep :type Boolean) (SweepResult :type Hit%20Result%20Structure%20%28by%20ref%29))
  ;[0.15 0.15 0.15 0.5] Close Target and Chest
  (Utilities|Casting|CastToBP_Arrow OtherActor
    (:then
      (Components|DestroyComponent (Variables|Default|GetTarget))
      ;[0.15 0.15 0.15 0.5] Open Chest and Spawn Target
      (bind _newtrack_0 (Timeline|TargetSpawn Reverse)
        (:Update
          (Transformation|SetRelativeLocation (Variables|Default|GetTarget) (Math|Vector|Lerp(Vector) "22.000000,45.000000,13.000000" "22.000000,45.000000,50.000000" _newtrack_0) false false))
        (:Finished
          (bind _returnvalue (Actor|GetActorOfClass "/Game/Blueprints/BP_Chest+TargetManager.BP_Chest+TargetManager_C"))
          (Default|RandomChest&Target _returnvalue))))
    (:CastFailed
      (Development|PrintString "NOOOOPE"))))

(event Custom|StartSequence
  ;[0.15 0.15 0.15 0.5] Open Chest and Spawn Target
  (Utilities|FlowControl|Delay 2.0)
  (bind _newtrack_0 (Timeline|Chest_Open Play)
    (:Update
      (Transformation|SetRelativeRotation (Variables|Default|GetTopChest) (Math|Rotator|Lerp(Rotator) "0.000000,0.000000,0.000000" "90.000000,0.000000,0.000000" _newtrack_0) false false))
    (:Finished
      (Utilities|FlowControl|Delay 5.0)
      (bind _newtrack_0_2 (Timeline|TargetSpawn Play)
        (:Update
          (Transformation|SetRelativeLocation (Variables|Default|GetTarget) (Math|Vector|Lerp(Vector) "22.000000,45.000000,13.000000" "22.000000,45.000000,50.000000" _newtrack_0_2) false false))
        (:Finished
          (bind _returnvalue (Actor|GetActorOfClass "/Game/Blueprints/BP_Chest+TargetManager.BP_Chest+TargetManager_C"))
          (Default|RandomChest&Target _returnvalue))))))

(fn ConstructionScript)