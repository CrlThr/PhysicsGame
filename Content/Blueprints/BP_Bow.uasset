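; Bow Blueprint that builds up shot power and fires BP_Arrow projectiles.
; ChargeBow grows ShootImpulse on each call by adding delta time and multiplying, clamped to a fixed range, so the growth is exponential and frame-rate dependent.
; Shoot spawns an arrow at the Arrow component's transform, applies the charge as a velocity-change impulse along the Bow's forward vector, prints debug values and resets the charge.
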(event Custom|Shoot
  ;[0.15 0.15 0.15 0.5] Shoot
  (Development|PrintString (Utilities|String|ToString(Float) (Variables|Default|GetShootImpulse)))
  (bind _returnvalue (Game|SpawnActorfromClass "/Game/Blueprints/BP_Arrow.BP_Arrow_C" (Transformation|GetWorldTransform (Variables|Default|GetArrow)) "Undefined" "MultiplyWithRoot" 0 0))
  (Development|PrintString (Utilities|String|ToString(Vector) (* (Variables|Default|GetShootImpulse) (Math|Vector|GetForwardVector (Variables|Actor|GetBow)))))
  (Physics|AddImpulse (Variables|/Game/Blueprints/BP_Arrow.BP_Arrow_C|GetArrow _returnvalue) (* (Variables|Default|GetShootImpulse) (Math|Vector|GetForwardVector (Variables|Actor|GetBow))) "None" true)
  (Variables|Default|SetShootImpulse 0.0))

(event Custom|ChargeBow
  ;[0.15 0.15 0.15 0.5] Shoot
  (Variables|Default|SetShootImpulse (Math|Float|Clamp(Float) (* (+ (Utilities|Time|GetWorldDeltaSeconds) (Variables|Default|GetShootImpulse)) 1.05) 7.5e+02 7e+03)))

(fn ConstructionScript)