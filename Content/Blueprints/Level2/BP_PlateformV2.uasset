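; BP_PlateformV2 is a Level 2 obstacle with a physics-driven swinging ball that knocks the player away on contact.
; Each tick, a sine of game time sets the PhysicsConstraint's angular orientation target, oscillating the ball in pitch.
; When the ball hits a BP_FirstPersonCharacter, its linear velocity is applied to the character's movement as a velocity-change impulse, ignoring mass.
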(event OnComponentHit(Ball)
  (params (HitComponent :type Primitive%20Component%20Object%20Reference) (OtherActor :type Actor%20Object%20Reference) (OtherComp :type Primitive%20Component%20Object%20Reference) (NormalImpulse :type Vector :default "0, 0, 0") (Hit :type Hit%20Result%20Structure%20%28by%20ref%29))
  ;[0.15 0.15 0.15 0.5] Eject the player
  (bind _asbp_first_person_character (Utilities|Casting|CastToBP_FirstPersonCharacter OtherActor))
  (bind _returnvalue (Physics|GetPhysicsLinearVelocity (Variables|Default|GetBall) "None"))
  (Physics|AddImpulse (Variables|/Script/Engine.Character|GetCharacterMovement _asbp_first_person_character) _returnvalue true))

(event EventTick
  (params (DeltaSeconds :type Float%20%28single-precision%29))
  ;[0.15 0.15 0.15 0.5] Move the ball
  (Class|PhysicsConstraintComponent|SetAngularOrientationTarget (Variables|Default|GetPhysicsConstraint) (Math|Rotator|MakeRotator 0.0 (* (Math|Trig|Sin(Radians) (* (Utilities|Time|GetGameTimeinSeconds) 2.0)) 8e+01) 0.0)))

(fn ConstructionScript)