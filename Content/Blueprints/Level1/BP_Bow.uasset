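; BP_Bow is the player's bow, which charges a shot and fires BP_Arrow projectiles, with UI events for a charge bar and crosshair.
; ChargeBow grows ShootImpulse each call by delta time and a multiplier, clamps it between Min and Max, and updates the progress bar.
; Shoot spawns an arrow at the Arrow component's transform, launches it along the bow's forward vector, resets the charge and gives it a limited lifespan.
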(event Custom|Shoot
  ;[0.15 0.15 0.15 0.5] Shoot
  (bind _returnvalue (Game|SpawnActorfromClass "/Game/Blueprints/Level1/BP_Arrow.BP_Arrow_C" (Transformation|GetWorldTransform (Variables|Default|GetArrow)) "Undefined" "MultiplyWithRoot" 0 0))
  (Physics|AddImpulse (Variables|/Game/Blueprints/Level1/BP_Arrow.BP_Arrow_C|GetArrow _returnvalue) (* (Variables|Default|GetShootImpulse) (Math|Vector|GetForwardVector (Variables|Actor|GetBow))) "None" true)
  (Variables|Default|SetShootImpulse 0.0)
  (Actor|SetLifeSpan _returnvalue 5.0))

(event Custom|ChargeBow
  (bind _max (Variables|Default|GetMax))
  (bind _min (Variables|Default|GetMin))
  ;[0.15 0.15 0.15 0.5] Shoot
  (bind _output_get (Variables|Default|SetShootImpulse (Math|Float|Clamp(Float) (* (+ (Utilities|Time|GetWorldDeltaSeconds) (Variables|Default|GetShootImpulse)) 1.05) _min _max)))
  (Default|SetIntensityShoot (Variables|Default|GetWBPBar) _output_get _min _max))

(event Custom|CreateUIBar
  ;[0.15 0.15 0.15 0.5] Create UI
  (bind _returnvalue (Game|ConstructObjectfromClass "/Game/Ui/WBP_ProgressBar.WBP_ProgressBar_C"))
  (Variables|Default|SetWBPBar _returnvalue)
  (Variables|Default|SetShootImpulse (Variables|Default|GetMin))
  (UserInterface|Viewport|AddtoViewport _returnvalue 0))

(event Custom|CreateUICrosshair
  ;[0.15 0.15 0.15 0.5] Create UI
  (bind _returnvalue (Game|ConstructObjectfromClass "/Game/Ui/WBP_Crosshair.WBP_Crosshair_C"))
  (Variables|Default|SetWBPCrosshair _returnvalue)
  (UserInterface|Viewport|AddtoViewport _returnvalue 0))

(fn ConstructionScript)