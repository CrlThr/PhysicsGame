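; BP_Door is a Level 1 door that opens once enough chest targets have been hit.
; Its Loop event scans the Chests array and decrements WinCondition for each BP_Chest with HitTarget set.
; At zero or below, OpenDoor slides the door between fixed world positions via a timeline-driven lerp.
; A second chest loop has an empty body, so TargetDown and ChestClose run after it, on a single element.
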(event Custom|OpenDoor
  ;[0.15 0.15 0.15 0.5] DoorTimeline
  (bind _newtrack_0 (Timeline|DoorTimeline Play)
    (:Update
      (Transformation|SetWorldLocation (Variables|Default|GetDoor) (Math|Vector|Lerp(Vector) "-2737.000000,-50.000000,203.000000" "-2737.000000,235.000000,203.000000" _newtrack_0) false false))))

(event Custom|Loop
  ;[0.15 0.15 0.15 0.5] Loop if we hit the target
  (for _array_element (Variables|Default|GetChests)
    (bind _asbp_chest (Utilities|Casting|CastToBP_Chest _array_element))
    (if (Variables|/Game/Blueprints/Level1/BP_Chest.BP_Chest_C|GetHit%20Target%20 _asbp_chest)
      (bind _output_get (Variables|Default|SetWin%20condition (- (Variables|Default|GetWin%20condition) 1)))
      (if (not (not (<= _output_get 0)))
        (CallFunction|OpenDoor)
        (for _array_element_2 (Variables|Default|GetChests)
          _)
        (bind _asbp_chest_2 (Utilities|Casting|CastToBP_Chest _array_element_2))
        (Default|TargetDown _asbp_chest_2)
        (Default|ChestClose _asbp_chest_2)))))

(fn ConstructionScript)