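; BP_FinalDoor is the Level 3 final door, which opens when three buttons are overlapped at the same time.
; The Loop event copies each Buttons element's IsOverlapping state into one of three index-specific flags, then calls OpenDoor if all three are true.
; OpenDoor plays a timeline that lerps the door upward between two hardcoded world positions.
; Nothing in this graph calls Loop.
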(event Custom|OpenDoor
  ;[0.15 0.15 0.15 0.5] DoorTimeline
  (bind _newtrack_0 (Timeline|Timeline Play)
    (:Update
      (Transformation|SetWorldLocation (Variables|Default|GetFinalDoor) (Math|Vector|Lerp(Vector) "-1200.000001,130.000004,-830.000000" "-1200.000001,130.000004,-170.000000" _newtrack_0) false false))))

(event Custom|Loop
  ;[0.15 0.15 0.15 0.5] Loop To Win
  (for (_array_element _array_index) (Variables|Default|GetButtons)
    (if (== _array_index 0)
      (Variables|Default|SetIs%20Button1Overlapping (Variables|/Game/Blueprints/Level3/BP_Button.BP_Button_C|GetIsOverlapping _array_element))
      (if (Math|Boolean|ANDBoolean (Variables|Default|GetIs%20Button1Overlapping) (Variables|Default|GetIs%20Button2Overlapping) (Variables|Default|GetIs%20Button3Overlapping)) :!label _label
        (CallFunction|OpenDoor))
      (elif (== _array_index 1)
        (Variables|Default|SetIs%20Button2Overlapping (Variables|/Game/Blueprints/Level3/BP_Button.BP_Button_C|GetIsOverlapping _array_element))
        (goto _label)
        (elif (== _array_index 2)
          (Variables|Default|SetIs%20Button3Overlapping (Variables|/Game/Blueprints/Level3/BP_Button.BP_Button_C|GetIsOverlapping _array_element))
          (goto _label))))))

(fn ConstructionScript)