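; BP_Button is a Level 3 pressure button that sinks when overlapped and signals the final door.
; BeginPlay stores its starting transform and a slightly lowered copy, which the PressButton timeline blends between, playing on overlap and reversing on end overlap.
; Every timeline update, in either direction, calls Loop on the FinalDoor reference cast to BP_FinalDoor, printing a debug string if the cast fails.
; An IsOverlapping flag tracks the overlap state.
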(event OnComponentBeginOverlap(Collision)
  (params (OverlappedComponent :type Primitive%20Component%20Object%20Reference) (OtherActor :type Actor%20Object%20Reference) (OtherComp :type Primitive%20Component%20Object%20Reference) (OtherBodyIndex :type Integer) (bFromSweep :type Boolean) (SweepResult :type Hit%20Result%20Structure%20%28by%20ref%29))
  ;[0.15 0.15 0.15 0.5] Button Press Timeline
  (Variables|Default|SetIsOverlapping true)
  (bind _newtrack_0 (Timeline|PressButton Play)
    (:Update
      (Transformation|SetActorTransform (Math|Transform|Lerp(Transform) (Variables|Default|GetOgTransform) (Variables|Default|GetNewTransform) _newtrack_0))
      (bind _asbp_final_door (Utilities|Casting|CastToBP_FinalDoor (Variables|Default|GetFinalDoor))
        (:then
          (Default|Loop _asbp_final_door))
        (:CastFailed
          (Development|PrintString "aaaaaaaaaa" true true "(R=1.000000,G=0.000000,B=0.000000,A=1.000000)"))))))

(event OnComponentEndOverlap(Collision)
  (params (OverlappedComponent :type Primitive%20Component%20Object%20Reference) (OtherActor :type Actor%20Object%20Reference) (OtherComp :type Primitive%20Component%20Object%20Reference) (OtherBodyIndex :type Integer))
  ;[0.15 0.15 0.15 0.5] Button Press Timeline
  (Variables|Default|SetIsOverlapping false)
  (bind _newtrack_0 (Timeline|PressButton Reverse)
    (:Update
      (Transformation|SetActorTransform (Math|Transform|Lerp(Transform) (Variables|Default|GetOgTransform) (Variables|Default|GetNewTransform) _newtrack_0))
      (bind _asbp_final_door (Utilities|Casting|CastToBP_FinalDoor (Variables|Default|GetFinalDoor))
        (:then
          (Default|Loop _asbp_final_door))
        (:CastFailed
          (Development|PrintString "aaaaaaaaaa" true true "(R=1.000000,G=0.000000,B=0.000000,A=1.000000)"))))))

(event EventBeginPlay
  ;[0.15 0.15 0.15 0.5] Get Button Location
  (bind _output_get (Variables|Default|SetOgTransform (Transformation|GetActorTransform)))
  (Variables|Default|SetNewTransform (Math|Transform|MakeTransform (+ (.location _output_get) "0.000000,0.000000,-10.000000") (.rotation _output_get) (.scale _output_get))))

(fn ConstructionScript)