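; Level 3 door actor that opens by becoming hidden and non-collidable when a button's OpenDoor flag is set.
; Each Tick it looks up a BP_Button_Child with GetActorOfClass and polls that flag, using IsActive to apply the closed, visible state only once.
; Opening also disables the actor's Tick, so its own polling stops and the closing branch no longer runs afterward.
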(event EventTick
  (params (DeltaSeconds :type Float%20%28single-precision%29))
  ;[0.15 0.15 0.15 0.5] Open the invisible Door
  (bind _returnvalue (Actor|GetActorOfClass "/Game/Blueprints/Level3/BP_Button_Child.BP_Button_Child_C"))
  (if (Variables|/Game/Blueprints/Level3/BP_Button_Child.BP_Button_Child_C|GetOpenDoor _returnvalue)
    (Rendering|SetActorHiddenInGame true)
    (Collision|SetActorEnableCollision false)
    (Actor|Tick|SetActorTickEnabled false)
    (Variables|Default|SetIsActive false)
    (elif (not (Variables|Default|GetIsActive))
      (Variables|Default|SetIsActive true)
      (Rendering|SetActorHiddenInGame false)
      (Collision|SetActorEnableCollision true)
      (Actor|Tick|SetActorTickEnabled true))))

(fn ConstructionScript)